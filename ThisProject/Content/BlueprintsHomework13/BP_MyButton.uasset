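; BP_MyButton is an interactable button actor that toggles its color when the player presses E nearby.
; Entering its box trigger enables input and shows a prompt widget; leaving disables input and hides it.
; On BeginPlay it applies a dynamic material instance to the button mesh, and each E press flip-flops that material's Color parameter between green and red.
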(event `self.ReceiveBeginPlay`
  (bind _returnvalue (`KismetMaterialLibrary.CreateDynamicMaterialInstance` "/Game/BlueprintsHomework13/M_ButtonColor.M_ButtonColor"))
  (bind _output_get (set `self.DynMaterial` _returnvalue))
  (`PrimitiveComponent.SetMaterial` (`self.ButtonMesh`) 0 _output_get))

(event `self.Box.OnComponentBeginOverlap`
  (params (OverlappedComponent :type "PrimitiveComponent Object Reference") (OtherActor :type "Actor Object Reference") (OtherComp :type "PrimitiveComponent Object Reference") (OtherBodyIndex :type Integer) (bFromSweep :type Boolean) (SweepResult :type "HitResult Structure (by ref)"))
  (`self.EnableInput` (`GameplayStatics.GetPlayerController` 0))
  (`SceneComponent.SetVisibility` (`self.Widget`) true false))

(event `self.Box.OnComponentEndOverlap`
  (params (OverlappedComponent :type "PrimitiveComponent Object Reference") (OtherActor :type "Actor Object Reference") (OtherComp :type "PrimitiveComponent Object Reference") (OtherBodyIndex :type Integer))
  (`self.DisableInput` (`GameplayStatics.GetPlayerController` 0))
  (`SceneComponent.SetVisibility` (`self.Widget`) false false))

(event `Key|E`
  (params (Key :type "Key Structure"))
  (bind _dynmaterial (`self.DynMaterial`))
  (:`Pressed`
    (`/Engine/EditorBlueprintResources/StandardMacros.FlipFlop`
      (:`A`
        (`MaterialInstanceDynamic.SetVectorParameterValue` _dynmaterial "Color" (struct :`R` 0.059141 :`G` 1.0 :`B` 0.087599 :`A` 1.0)))
      (:`B`
        (`MaterialInstanceDynamic.SetVectorParameterValue` _dynmaterial "Color" (struct :`R` 1.0 :`G` 0.005606 :`B` 0.032348 :`A` 1.0))))))

(fn `UserConstructionScript`)