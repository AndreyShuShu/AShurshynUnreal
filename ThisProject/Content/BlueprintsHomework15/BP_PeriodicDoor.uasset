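; Periodic door actor that swings open and closed on its own in a repeating cycle, starting at BeginPlay.
; DoorMoveTimeline drives the DoorHinge yaw between zero and OpenAngle, playing forward to open and reversing to close.
; When the timeline finishes, it waits WaitTime, then a FlipFlop selects opening or closing.
; The FlipFlop's first output is opening, so the first pass calls open again on the already open door.
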(event `StartOpening`
  (bind (_direction _alpha) (`Timeline|DoorMoveTimeline` :!label _label)
    (:`Update`
      (`SceneComponent.K2_SetRelativeRotation` (`self.DoorHinge`) (`KismetMathLibrary.MakeRotator` 0.0 0.0 (`KismetMathLibrary.Lerp` 0.0 (`self.OpenAngle`) _alpha)) false false))
    (:`Finished`
      (`KismetSystemLibrary.Delay` (`self.WaitTime`))
      (`/Engine/EditorBlueprintResources/StandardMacros.FlipFlop`
        (:`A`
          (`self.StartOpening`))
        (:`B`
          (`self.StartClosing`))))))

(event `StartClosing`
  (goto _label :!via `Reverse`))

(event `self.ReceiveBeginPlay`
  (`self.StartOpening`))

(fn `UserConstructionScript`)