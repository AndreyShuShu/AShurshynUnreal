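; Health platform actor that jumps around a square path and changes the player's health on contact.
; From BeginPlay, an endless loop offsets the actor along X and Y to each corner in turn, pausing on a Delay between instant, non-swept jumps.
; When its Box component begins overlapping a NewCharacter, it calls that character's UpdateHealth with a fixed positive amount.
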(event `self.ReceiveBeginPlay`
  (`self.K2_AddActorWorldOffset` (800.0 0.0 0.0) :!label _label)
  (`KismetSystemLibrary.Delay` 1.0)
  (`self.K2_AddActorWorldOffset` (0.0 800.0 0.0))
  (`KismetSystemLibrary.Delay` 1.0)
  (`self.K2_AddActorWorldOffset` (-800.0 0.0 0.0))
  (`KismetSystemLibrary.Delay` 1.0)
  (`self.K2_AddActorWorldOffset` (0.0 -800.0 0.0))
  (`KismetSystemLibrary.Delay` 1.0)
  (goto _label))

(event `self.Box.OnComponentBeginOverlap`
  (params (OverlappedComponent :type "PrimitiveComponent Object Reference") (OtherActor :type "Actor Object Reference") (OtherComp :type "PrimitiveComponent Object Reference") (OtherBodyIndex :type Integer) (bFromSweep :type Boolean) (SweepResult :type "HitResult Structure (by ref)"))
  (bind _asnew_character (cast `/Game/Blueprints/NewCharacter` OtherActor))
  (`/Game/Blueprints/NewCharacter.UpdateHealth` _asnew_character 5.0))

(fn `UserConstructionScript`)