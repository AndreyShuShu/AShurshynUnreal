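; Damage platform actor that moves in a horizontal circle and hurts the player on contact.
; Tick repositions it around its BeginPlay location using sine and cosine of game time scaled by a rotation speed and radius, without sweeping.
; When its Sphere component begins overlapping a NewCharacter, it applies negative health through that character's UpdateHealth.
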(event `self.ReceiveBeginPlay`
  (set `self.InitialLocation` (`self.K2_GetActorLocation`)))

(event `self.ReceiveTick`
  (params (DeltaSeconds :type "Float (single-precision)"))
  (bind _radius (`self.Radius`))
  (bind _returnvalue (* (`KismetSystemLibrary.GetGameTimeInSeconds`) (`self.RotationSpeed`)))
  (`self.K2_SetActorLocation` (`KismetMathLibrary.MakeVector` (+ (.x (`self.InitialLocation`)) (* _radius (`KismetMathLibrary.DegCos` _returnvalue))) (+ (.y (`self.InitialLocation`)) (* (`KismetMathLibrary.DegSin` _returnvalue) _radius)) (.z (`self.InitialLocation`)))))

(event `self.Sphere.OnComponentBeginOverlap`
  (params (OverlappedComponent :type "PrimitiveComponent Object Reference") (OtherActor :type "Actor Object Reference") (OtherComp :type "PrimitiveComponent Object Reference") (OtherBodyIndex :type Integer) (bFromSweep :type Boolean) (SweepResult :type "HitResult Structure (by ref)"))
  (bind _asnew_character (cast `/Game/Blueprints/NewCharacter` OtherActor))
  (`/Game/Blueprints/NewCharacter.UpdateHealth` _asnew_character -5.0))

(fn `UserConstructionScript`)